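; AI hand pawn that flees from pawns it sees by moving to tagged escape points.
; On PawnSensing sight, it picks the "HandPoint" actor closest to itself among those outside a radius around the seen pawn, then uses AIMoveTo, with debug prints during the search.
; A looping random Roam event exists, but BeginPlay is empty and nothing live here starts it.
; The furthest-point search is left disconnected.
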(event OnSeePawn(PawnSensing)
  (params (Pawn :type Pawn%20Object%20Reference))
  (bind _self self)
  (Utilities|FlowControl|Sequence
    (:then_0
      (bind _goto (CallFunction|GetNearestPointNotinRadius _self Pawn 2e+03))
      (AI|AIMoveTo _self "0, 0, 0" _goto 5.0 false))))

(event Custom|Roam
  (AI|AIMoveTo self (.RandomLocation (AI|Navigation|GetRandomReachablePointinRadius (Transformation|GetActorLocation) 2e+03 0 0)) 0 5.0 false
    (:OnSuccess
      _)
    (:OnFail
      _))
  (CallFunction|Roam))

(event EventBeginPlay)

(fn ConstructionScript)

(fn GetFurthestPoint
  (params (Player :type Pawn%20Object%20Reference))
  (bind _outactors (Actor|GetAllActorswithTag "HandPoint"))
  (for _array_element _outactors
    (if (< (LocalVariables|GetDistanceFromPoint) (Transformation|GetDistanceTo _array_element Player))
      (LocalVariables|SetDistanceFromPoint (Transformation|GetDistanceTo _array_element Player))
      (LocalVariables|SetGo%20To _array_element)))
  (return (LocalVariables|GetGo%20To)))

(fn GetNearestPointNotinRadius
  (params (Player :type Pawn%20Object%20Reference) (Radius :type Float%20%28double-precision%29))
  (bind _outactors (Actor|GetAllActorswithTag "HandPoint"))
  (for _array_element _outactors
    ;[1 1 1] if (pointFromPlayer > radius)
    (Development|PrintString (Utilities|String|ToString(Float) (Transformation|GetDistanceTo _array_element Player)))
    (if (< Radius (Transformation|GetDistanceTo _array_element Player))
      ;[1 1 1] if (distanceFromCurrentPoint > distanceFromPoint) {set this point as current}
      (if (> (LocalVariables|GetDistanceFromPoint) (Transformation|GetDistanceTo _array_element self))
        (Development|PrintString (Utilities|GetDisplayName (LocalVariables|GetGo%20To)))
        (LocalVariables|SetDistanceFromPoint (Transformation|GetDistanceTo _array_element self))
        (LocalVariables|SetGo%20To _array_element))))
  (return (LocalVariables|GetGo%20To)))