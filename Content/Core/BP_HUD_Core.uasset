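; Core HUD Blueprint that creates the game HUD and inventory widgets and adds them to the viewport on BeginPlay.
; Menus register in a GameMenus array, so ToggleWidget can collapse the other menus when one is toggled, as toggleInventory does for the inventory.
; ChangeHudMode flips the active menu's visibility, switching between game-only and game-and-UI input along with the mouse cursor.
; Outline material code in ChangeHudMode is disconnected and never runs.
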(event Custom|toggleInventory
  (CallFunction|ToggleWidget (Variables|Default|GetWB_Inventory)))

(event EventBeginPlay
  (Input|SetInputModeGameOnly (Game|GetPlayerController 0) false)
  ;[0.2655 1 0.5793] Game
  (bind _returnvalue (UserInterface|CreateWidget "/Game/Core/WB_HUD.WB_HUD_C" (Game|GetPlayerController 0)))
  (bind _output_get (Variables|Default|SetWB_HUD _returnvalue))
  (UserInterface|Viewport|AddtoViewport _output_get 0)
  ;[1 1 1] Game Menu's
  (Utilities|FlowControl|Sequence
    (:then_0
      (bind _returnvalue_2 (UserInterface|CreateWidget "/Game/Core/WB_Inventory.WB_Inventory_C" (Game|GetPlayerController 0)))
      (bind _output_get_2 (Variables|Default|SetWB_Inventory _returnvalue_2))
      (Utilities|Array|Add (Variables|Default|GetGameMenus) _output_get_2))
    (:then_2
      (for _array_element (Variables|Default|GetGameMenus)
        (UserInterface|Viewport|AddtoViewport _array_element 0)))))

(event Collision|EventActorBeginOverlap
  (params (OtherActor :type Actor%20Object%20Reference)))

(event EventTick
  (params (DeltaSeconds :type Float%20%28single-precision%29)))

(fn ConstructionScript)

(fn ToggleWidget
  (params (target%20widget :type User%20Widget%20Object%20Reference))
  (Utilities|IsValid target%20widget
    (:Is%20Valid
      (Variables|Default|SetActiveWidget target%20widget)
      (for _array_element (Variables|Default|GetGameMenus)
        (Utilities|IsValid _array_element
          (:Is%20Valid
            (if (== (Variables|Default|GetActiveWidget) _array_element)
              (CallFunction|ChangeHudMode)
              (elif (Widget|IsVisible _array_element)
                (Widget|SetVisibility _array_element "Collapsed")))))))))

(fn ChangeHudMode
  (bind _returnvalue (Game|GetPlayerController 0))
  (bind _activewidget (Variables|Default|GetActiveWidget))
  (if (Widget|IsVisible _activewidget)
    (Widget|SetVisibility _activewidget "Collapsed")
    (Input|SetInputModeGameOnly _returnvalue false)
    (Variables|/Script/Engine.PlayerController|SetbShowMouseCursor _returnvalue false)
    (else
      (Widget|SetVisibility _activewidget "Visible")
      (Input|SetInputModeGameandUI _returnvalue _activewidget "LockAlways" true false)
      (Variables|/Script/Engine.PlayerController|SetbShowMouseCursor _returnvalue true))))