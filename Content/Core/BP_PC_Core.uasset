(event EventBeginPlay
  (bind _asbp_hud_core (Utilities|GetPBHUD 1e+01)
    (:Success
      (Variables|Default|SetAs%20BP%20HUD%20Core _asbp_hud_core))))

(event Input|KeyboardEvents|Q
  (params (Key :type Key%20Structure :default "None"))
  ;[1 0.1354 0.3796] Drop Item
  (:Pressed
    (Default|DropCurrentHand (Actor|GetComponentbyClass (Pawn|GetControlledPawn) "/Game/Interaction/AC_InteractionTrace.AC_InteractionTrace_C"))))

(event Input|KeyboardEvents|I
  (params (Key :type Key%20Structure :default "None"))
  ;[0.3823 1 0.6428 0.692] Inventory toggle
  (:Pressed
    (Default|ToggleInventory (Variables|Default|GetAs%20BP%20HUD%20Core))))

(event Input|KeyboardEvents|E
  (params (Key :type Key%20Structure :default "None"))
  (bind _returnvalue (Pawn|GetControlledPawn))
  (bind _returnvalue_2 (Actor|GetComponentbyClass _returnvalue "/Game/Interaction/AC_InteractionTrace.AC_InteractionTrace_C"))
  ;[1 0.6119 0.02812 0.538] Interact with smth.
  (:Pressed
    (Default|TrytoInteract _returnvalue_2 true))
  (:Released
    (Default|TrytoInteract _returnvalue_2 false)))

(event Input|KeyboardEvents|V
  (params (Key :type Key%20Structure :default "None"))
  (bind _returnvalue (Game|GetGameMode))
  (bind _hudclass (Variables|/Script/Engine.GameModeBase|GetHUDClass _returnvalue))
  (:Pressed
    (bind _returnvalue_2 (Actor|GetActorOfClass _hudclass))
    (bind _asbp_hud_core (Utilities|Casting|CastToBP_HUD_Core _returnvalue_2))
    (Default|SetHUDVisibility _asbp_hud_core true))
  (:Released
    (bind _returnvalue_3 (Actor|GetActorOfClass _hudclass))
    (bind _asbp_hud_core_2 (Utilities|Casting|CastToBP_HUD_Core _returnvalue_3))
    (Default|SetHUDVisibility _asbp_hud_core_2 false)))

(fn ConstructionScript)