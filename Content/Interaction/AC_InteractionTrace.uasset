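; Player interaction component that drives swappable hands, whose abilities gate what the player can use.
; A per-tick camera line trace focuses BP_InteractionArea targets.
; Cooldown-gated interaction checks required abilities by set intersection, then swaps in a BP_HandObject or calls the target's Interact; without a target, it can toggle the character's glow light.
; Hands load mesh, abilities and cooldown from DataTable rows, respawn as pickups when dropped, and update HUD icon, progress and warnings.
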(event Custom|try%20to%20interact
  (params (In :type Boolean))
  (bind _abilitycooldown (Variables|Default|GetabilityCooldown))
  (bind _focusedinteractionarea (Variables|Default|GetFocusedInteractionArea))
  (bind _returnvalue (Actor|GetAttachParentActor _focusedinteractionarea))
  (if In
    (Utilities|FlowControl|DoOnce false :!label _label
      (:Completed
        (if (== 0.0 _abilitycooldown)
          (Utilities|FlowControl|Sequence
            (:then_0
              (goto _label Reset))
            (:then_1
              _))
          (else
            (bind _returnvalue_2 (Utilities|Time|SetTimerbyEvent (delegate Custom|CustomEvent) _abilitycooldown))))
        (if (Variables|Default|GetIsTracingInteractionArea)
          (bind _returnvalue_3 (CallFunction|DoesContainRequiredAbilities))
          (if _returnvalue_3
            (CallFunction|WarningMSGUI)
            (Variables|Default|SetsumCooldown 0.0)
            ;[1 0.9162 0.4732 0.271] not implemented - probably not needed
            (bind _output_get (Variables|Default|SetInteraction%20Duration (Variables|/Game/Interaction/InteractionArea/BP_InteractionArea.BP_InteractionArea_C|GetInteraction%20Duration (Variables|Default|GetFocusedInteractionArea))))
            (if (not (> _output_get 0.0))
              (bind _asbp_hand_object (Utilities|Casting|CastToBP_HandObject _returnvalue)
                (:then
                  (CallFunction|DropHand)
                  (bind _output_get_2 (Variables|Default|Setequipped%20Hand%20Data%20Row (Variables|/Game/Interaction/EquipmentSystem/BP_HandObject.BP_HandObject_C|GethandData _asbp_hand_object)))
                  (CallFunction|PickupNewHand _output_get_2)
                  ;[1 0 0.04179 0.454] Destroy The Hand Object after picking it up
                  (Variables|Default|SetIsTracingInteractionArea false)
                  (Actor|DestroyActor _returnvalue))
                (:CastFailed
                  ;[0.6028 1 0.6399] Other interactions
                  (Default|Interact (Variables|/Game/Interaction/InteractionArea/BP_InteractionArea.BP_InteractionArea_C|Gettarget%20interaction (Variables|Default|GetFocusedInteractionArea))))))
            (else
              (CallFunction|WarningMSGUI "You are missing required abilities to use this item!")))
          (else
            (CallFunction|HandyAbility)))))))

(event Custom|CustomEvent
  (bind _abilitycooldown (Variables|Default|GetabilityCooldown))
  (bind _focusedinteractionarea (Variables|Default|GetFocusedInteractionArea))
  (bind _returnvalue (Actor|GetAttachParentActor _focusedinteractionarea))
  (Utilities|Time|ClearandInvalidateTimerbyHandle (stale Custom|try%20to%20interact _returnvalue_2))
  (Utilities|FlowControl|DoOnce false) ; enters at Reset
)

(event Custom|Drop%20Current%20Hand
  (CallFunction|DropHand))

(event EventBeginPlay
  (CallFunction|PickupNewHand (Variables|Default|Getequipped%20Hand%20Data%20Row)))

(event EventTick
  (params (DeltaSeconds :type Float%20%28single-precision%29))
  (CallFunction|Trace)
  (if (< (Variables|Default|GetsumCooldown) (Variables|Default|GetabilityCooldown))
    (Variables|Default|SetsumCooldown (+ DeltaSeconds (Variables|Default|GetsumCooldown)))
    (if (< (Variables|Default|GetsumCooldown) (Variables|Default|GetabilityCooldown))
      (CallFunction|UpdateIconMaterialProgress (/ (Variables|Default|GetsumCooldown) (Variables|Default|GetabilityCooldown))))))

(fn Trace
  (bind _returnvalue (Game|GetPlayerCameraManager 0))
  (bind _returnvalue_2 (Transformation|GetActorLocation _returnvalue))
  (bind (_outhit _returnvalue_3) (Collision|LineTraceByChannel _returnvalue_2 (+ _returnvalue_2 (* (Math|Vector|GetForwardVector (Transformation|GetActorRotation _returnvalue)) (Variables|Default|Getlength))) "TraceTypeQuery1" false 0 "None"))
  (if _returnvalue_3
    (if (!= (Variables|Default|GetFocused%20Actor) (.HitActor (Collision|BreakHitResult _outhit)))
      (Variables|Default|SetFocused%20Actor (.HitActor (Collision|BreakHitResult _outhit)))
      (CallFunction|TraceInteractionArea (== "/Game/Interaction/InteractionArea/BP_InteractionArea.BP_InteractionArea_C" (Utilities|GetClass (.HitActor (Collision|BreakHitResult _outhit))))))
    (else
      (CallFunction|TraceInteractionArea false))))

(fn TraceInteractionArea
  (params (Trace :type Boolean))
  (if Trace
    (if (Variables|Default|GetIsTracingInteractionArea)
      (Default|ToggleFocus (Variables|Default|GetFocusedInteractionArea) false))
    (bind _asbp_interaction_area (Utilities|Casting|CastToBP_InteractionArea (Variables|Default|GetFocused%20Actor)))
    (bind _output_get (Variables|Default|SetFocusedInteractionArea _asbp_interaction_area))
    (Default|ToggleFocus _output_get true)
    (Variables|Default|SetIsTracingInteractionArea true)
    (elif (Variables|Default|GetIsTracingInteractionArea)
      (Variables|Default|SetIsTracingInteractionArea false)
      (Default|ToggleFocus (Variables|Default|GetFocusedInteractionArea) false)
      (Variables|Default|SetFocused%20Actor 0)
      (Variables|Default|SetFocusedInteractionArea 0))))

(fn DoesContainRequiredAbilities
  (bind _focusedinteractionarea (Variables|Default|GetFocusedInteractionArea))
  (bind _requiredabilities (Variables|/Game/Interaction/InteractionArea/BP_InteractionArea.BP_InteractionArea_C|GetRequiredAbilities _focusedinteractionarea))
  (bind _result (Utilities|Set|Intersection (Variables|Default|GetCurrent%20Abilities) _requiredabilities))
  (return (== (Utilities|Set|Length _result) (Utilities|Set|Length _requiredabilities))))

(fn PickupNewHand
  (params (Hand%20Data%20Row :type Data%20Table%20Row%20Handle%20Structure))
  ;[0.9934 0.4338 1] Hand Item Interaction
  (Utilities|FlowControl|Sequence
    (:then_0
      (bind _returnvalue (Utilities|GetDataTableRow (.datatable Hand%20Data%20Row) (.rowname Hand%20Data%20Row))
        (:then
          ;[1 1 1] Save its mesh to the players hand
          (bind _asbp_main_character (Utilities|Casting|CastToBP_MainCharacter (Components|GetOwner)))
          (Components|StaticMesh|SetStaticMesh (Variables|/Game/Characters/BP_MainCharacter.BP_MainCharacter_C|GetHand _asbp_main_character) (.StaticMesh (Utilities|Struct|BreakS_Hands _returnvalue)))
          (Variables|Default|SetCurrent%20Abilities (.Abilities (Utilities|Struct|BreakS_Hands _returnvalue)))
          (Variables|Default|SetabilityCooldown (.Cooldown (Utilities|Struct|BreakS_Hands _returnvalue)))
          ;[0.935 1 0.4409] add its name and icon to the HUD widget
          (bind _returnvalue_2 (Actor|GetActorOfClass (Variables|/Script/Engine.GameModeBase|GetHUDClass (Game|GetGameMode))))
          (bind _asbp_hud_core (Utilities|Casting|CastToBP_HUD_Core _returnvalue_2))
          (Variables|/Game/Core/WB_HUD.WB_HUD_C|SetHand_Name (Variables|/Game/Core/BP_HUD_Core.BP_HUD_Core_C|GetWB_HUD _asbp_hud_core) (.DisplayName (Utilities|Struct|BreakS_Hands _returnvalue)))
          (Default|SetHandIcon (Variables|/Game/Core/BP_HUD_Core.BP_HUD_Core_C|GetWB_HUD _asbp_hud_core) (.Icon (Utilities|Struct|BreakS_Hands _returnvalue)) (.Tint (Utilities|Struct|BreakS_Hands _returnvalue))))))
    (:then_1
      ;[1 0.9008 0.3665] stop Glowing
      (if (Utilities|IsValid _asbp_main_character)
        (Rendering|SetVisibility (Variables|/Game/Characters/BP_MainCharacter.BP_MainCharacter_C|GetGlowLightSource _asbp_main_character) false false)))))

(fn HandyAbility
  (Utilities|FlowControl|Sequence
    (:then_0
      (if (Utilities|Set|Contains (Variables|Default|GetCurrent%20Abilities) "NewEnumerator1")
        (bind _asbp_main_character (Utilities|Casting|CastToBP_MainCharacter (Components|GetOwner)))
        (Rendering|SetVisibility (Variables|/Game/Characters/BP_MainCharacter.BP_MainCharacter_C|GetGlowLightSource _asbp_main_character) (not (Rendering|IsVisible (Variables|/Game/Characters/BP_MainCharacter.BP_MainCharacter_C|GetGlowLightSource _asbp_main_character))) false)
        (CallFunction|UpdateIconMaterialProgress (Math|Conversions|ToFloat(Boolean) (Rendering|IsVisible (Variables|/Game/Characters/BP_MainCharacter.BP_MainCharacter_C|GetGlowLightSource _asbp_main_character))))))))

(fn UpdateIconMaterialProgress
  (params (progress :type Float%20%28double-precision%29))
  (bind _returnvalue (Actor|GetActorOfClass (Variables|/Script/Engine.GameModeBase|GetHUDClass (Game|GetGameMode))))
  (bind _asbp_hud_core (Utilities|Casting|CastToBP_HUD_Core _returnvalue))
  (Rendering|Material|SetScalarParameterValue (Variables|/Game/Core/WB_HUD.WB_HUD_C|GetHand_Icon_Material_Instance (Variables|/Game/Core/BP_HUD_Core.BP_HUD_Core_C|GetWB_HUD _asbp_hud_core)) "Usage" progress :!class /Script/Engine.MaterialInstanceDynamic)
  (Variables|/Game/Core/WB_HUD.WB_HUD_C|Setslate%20brush (Variables|/Game/Core/BP_HUD_Core.BP_HUD_Core_C|GetWB_HUD _asbp_hud_core) (Utilities|Struct|MakeSlateBrush "Image" "NoTile" "NoMirror" "(X=32.000000,Y=32.000000)" "(Left=0.000000,Top=0.000000,Right=0.000000,Bottom=0.000000)" "(SpecifiedColor=(R=1.000000,G=1.000000,B=1.000000,A=1.000000),ColorUseRule=UseColor_Specified)" "(CornerRadii=(X=0.000000,Y=0.000000,Z=0.000000,W=1.000000),Color=(SpecifiedColor=(R=0.000000,G=0.000000,B=0.000000,A=0.000000),ColorUseRule=UseColor_Specified),Width=0.000000,RoundingType=HalfHeightRadius,bUseBrushTransparency=False)" (Variables|/Game/Core/WB_HUD.WB_HUD_C|GetHand_Icon_Material_Instance (Variables|/Game/Core/BP_HUD_Core.BP_HUD_Core_C|GetWB_HUD _asbp_hud_core)))))

(fn WarningMSGUI
  (params (Warning :type String))
  (bind _returnvalue (Actor|GetActorOfClass (Variables|/Script/Engine.GameModeBase|GetHUDClass (Game|GetGameMode))))
  (bind _asbp_hud_core (Utilities|Casting|CastToBP_HUD_Core _returnvalue))
  (Default|HUDWarningMessage (Variables|/Game/Core/BP_HUD_Core.BP_HUD_Core_C|GetWB_HUD _asbp_hud_core) Warning 5.0))

(fn DropHand
  (if (!= (.rowname (Variables|Default|Getequipped%20Hand%20Data%20Row)) "No_Hand")
    (bind _asbp_main_character (Utilities|Casting|CastToBP_MainCharacter (Components|GetOwner)))
    (Game|SpawnActorfromClass "/Game/Interaction/EquipmentSystem/BP_HandObject.BP_HandObject_C" (Math|Transform|MakeTransform (Transformation|GetWorldLocation (Variables|/Game/Characters/BP_MainCharacter.BP_MainCharacter_C|GetSpringArm _asbp_main_character)) "0, 0, 0" "1.000000,1.000000,1.000000") "Undefined" "MultiplyWithRoot" 0 (Variables|Default|Getequipped%20Hand%20Data%20Row) 0)
    (bind _output_get (Variables|Default|Setequipped%20Hand%20Data%20Row (Utilities|Struct|MakeDataTableRowHandle "/Game/Interaction/EquipmentSystem/DT_Hands.DT_Hands" "No_Hand")))
    (CallFunction|PickupNewHand _output_get)))