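; Hand lever light child Blueprint that shows an on/off state through an emissive material on its Cube mesh.
; BeginPlay creates a dynamic instance of Switch_emit_light_Inst, applies it to Cube, and calls SwitchEmission if StartingValue is true.
; SwitchEmission flips CurrentState and writes it to the is_active scalar parameter.
; The Interact call in this graph is unwired, so only BeginPlay triggers the switch here.
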(event EventBeginPlay
  (bind _returnvalue (Rendering|Material|CreateDynamicMaterialInstance "/Game/Interaction/switch_emit_light_Inst.switch_emit_light_Inst" "None" "None" :!class /Script/Engine.KismetMaterialLibrary))
  (bind _output_get (Variables|Default|Setemission_DynMatInst _returnvalue))
  (Rendering|Material|SetMaterial (Variables|Default|GetCube) 0 _output_get)
  (if (Variables|Default|GetStartingValue)
    (CallFunction|SwitchEmission)))

(fn ConstructionScript
  (|CallParentFunction))

(fn SwitchEmission
  (Variables|Default|SetCurrentState (not (Variables|Default|GetCurrentState)))
  (Rendering|Material|SetScalarParameterValue (Variables|Default|Getemission_DynMatInst) "is_active" (Math|Conversions|ToFloat(Boolean) (Variables|Default|GetCurrentState)) :!class /Script/Engine.MaterialInstanceDynamic))