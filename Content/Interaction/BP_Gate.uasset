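; BP_Gate is an interactable gate that slides between its starting location and an offset position.
; BeginPlay stores the start as PositionA, and PositionB serves as an offset relative to it.
; Each PrimaryInteract alternates through a FlipFlop between playing and reversing a Timeline that lerps the actor's location without sweep.
; A DoOnce, reset when the Timeline finishes, blocks retriggering during movement.
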(event EventPrimaryInteract
  (bind _position_a (Variables|Default|GetPosition%20A))
  (Utilities|FlowControl|DoOnce false :!label _label
    (:Completed
      (Utilities|FlowControl|FlipFlop
        (:A
          (bind _newtrack_0 (Timeline|Timeline Play)
            (:Update
              (Transformation|SetActorLocation (Math|Vector|Lerp(Vector) _position_a (+ _position_a (Variables|Default|GetPosition%20B)) _newtrack_0) false false))
            (:Finished
              (goto _label Reset))))
        (:B
          (Timeline|Timeline Reverse))))))

(event EventInteract)

(event EventBeginPlay
  (Variables|Default|SetPosition%20A (Transformation|GetActorLocation)))

(fn ConstructionScript
  (|CallParentFunction))