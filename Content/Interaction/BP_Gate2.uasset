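; BP_Gate2 is an interactable gate that slides between its starting location and an offset position.
; BeginPlay stores the start location, and a Timeline lerps the actor from there to that point plus PositionB, without sweeping.
; Each accepted Interact flips between playing and reversing the Timeline.
; A DoOnce blocks further interaction until the Timeline finishes and resets it.
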(event EventInteract
  (bind _positiona (Variables|Default|GetPositionA))
  (Utilities|FlowControl|DoOnce false :!label _label
    (:Completed
      (Utilities|FlowControl|FlipFlop
        (:A
          (bind _newtrack_0 (Timeline|Timeline Play)
            (:Update
              (Transformation|SetActorLocation (Math|Vector|Lerp(Vector) _positiona (+ _positiona (Variables|Default|GetPositionB)) _newtrack_0) false false))
            (:Finished
              (goto _label Reset))))
        (:B
          (Timeline|Timeline Reverse))))))

(event EventBeginPlay
  (Variables|Default|SetPositionA (Transformation|GetActorLocation)))

(fn ConstructionScript
  (|CallParentFunction))