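; BP_GateWithTimer is an interactable gate that slides open on interaction and closes itself after a delay.
; Interact cancels any pending close timer and plays a timeline that lerps the actor from its BeginPlay location to that location plus the PositionB offset.
; EndInteract starts a one-shot timer of DelayBeforeClosing, after which the timeline reverses to close the gate.
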(event Custom|AfterEndInteractTimerEvent
  (bind _positiona (Variables|Default|GetPositionA))
  (Utilities|Time|ClearandInvalidateTimerbyHandle (stale EventEndInteract _returnvalue))
  (bind _newtrack_0 (Timeline|Timeline Reverse)
    (:Update
      (Transformation|SetActorLocation (Math|Vector|Lerp(Vector) _positiona (+ _positiona (Variables|Default|GetPositionB)) _newtrack_0) false false))))

(event EventEndInteract
  (bind _returnvalue (Utilities|Time|SetTimerbyEvent (delegate Custom|AfterEndInteractTimerEvent) (Variables|Default|GetDelayBeforeClosing))))

(event EventInteract
  (bind _positiona (Variables|Default|GetPositionA))
  (Utilities|Time|ClearandInvalidateTimerbyHandle (stale EventEndInteract _returnvalue))
  (bind _newtrack_0 (Timeline|Timeline Play)
    (:Update
      (Transformation|SetActorLocation (Math|Vector|Lerp(Vector) _positiona (+ _positiona (Variables|Default|GetPositionB)) _newtrack_0) false false))))

(event EventBeginPlay
  (Variables|Default|SetPositionA (Transformation|GetActorLocation)))

(fn ConstructionScript
  (|CallParentFunction))