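; Switchable point light actor that toggles the visibility of its PointLight component on Interact, starting from a configurable default state.
; On BeginPlay it gives the light a dynamic instance of a flickering light function material, with a random BlinkOffset so each light blinks out of sync.
; A SwitchOnlyOnce flag routes Interact through a DoOnce node, and Tick checks visibility without acting on it.
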(event EventBeginPlay
  (Development|SetHiddeninGame (Variables|Default|GetPointLight) (Variables|Default|GetDefaultHiddenInGame) false)
  (bind _returnvalue (Rendering|Material|CreateDynamicMaterialInstance "/Game/materials/flickeringLightFunction.flickeringLightFunction" "None" "None" :!class /Script/Engine.KismetMaterialLibrary))
  (Rendering|Material|SetScalarParameterValue _returnvalue "BlinkOffset" (* (Math|Random|RandomFloat) 1e+02) :!class /Script/Engine.MaterialInstanceDynamic)
  (Rendering|Components|Light|SetLightFunctionMaterial (Variables|Default|GetPointLight) _returnvalue))

(event EventTick
  (params (DeltaSeconds :type Float%20%28single-precision%29))
  (if (not (Variables|/Script/Engine.SceneComponent|GetbHiddenInGame (Variables|Default|GetPointLight)))
    _))

(event EventInteract
  (bind _pointlight (Variables|Default|GetPointLight))
  (if (Variables|Default|GetswitchOnlyOnce)
    (Utilities|FlowControl|DoOnce false
      (:Completed
        _)))
  (Development|SetHiddeninGame _pointlight (not (Variables|/Script/Engine.SceneComponent|GetbHiddenInGame _pointlight)) false))

(fn ConstructionScript
  (|CallParentFunction))