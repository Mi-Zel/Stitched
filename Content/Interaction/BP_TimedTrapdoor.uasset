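; Timed trapdoor actor that opens when interacted with and closes again after a delay once interaction ends.
; Interact cancels any pending close timer and plays a Timeline that lerps the actor from its BeginPlay transform toward TransformB.
; TransformB's location and rotation are offsets added to the starting transform, while its scale is absolute.
; EndInteract starts the DelayBeforeClosing timer, which reverses the Timeline.
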(event Custom|AfterEndInteractTimerEvent
  (bind _transformb (Variables|Default|GetTransformB))
  (bind _transforma (Variables|Default|GetTransformA))
  (bind (_roll _pitch _yaw) (Math|Rotator|BreakRotator (.rotation _transformb)))
  (bind (_roll_2 _pitch_2 _yaw_2) (Math|Rotator|BreakRotator (.rotation _transforma)))
  (Utilities|Time|ClearandInvalidateTimerbyHandle (stale EventEndInteract _returnvalue))
  (bind _newtrack_0 (Timeline|Timeline Reverse)
    (:Update
      (Transformation|SetActorTransform (Math|Transform|Lerp(Transform) (Variables|Default|GetTransformA) (Math|Transform|MakeTransform (+ (.location _transformb) (.location _transforma)) (Math|Rotator|MakeRotator (+ _roll _roll_2) (+ _pitch _pitch_2) (+ _yaw _yaw_2)) (.scale _transformb)) _newtrack_0)))))

(event EventEndInteract
  (bind _returnvalue (Utilities|Time|SetTimerbyEvent (delegate Custom|AfterEndInteractTimerEvent) (Variables|Default|GetDelayBeforeClosing))))

(event EventInteract
  (bind _transformb (Variables|Default|GetTransformB))
  (bind _transforma (Variables|Default|GetTransformA))
  (bind (_roll _pitch _yaw) (Math|Rotator|BreakRotator (.rotation _transformb)))
  (bind (_roll_2 _pitch_2 _yaw_2) (Math|Rotator|BreakRotator (.rotation _transforma)))
  (Utilities|Time|ClearandInvalidateTimerbyHandle (stale EventEndInteract _returnvalue))
  (bind _newtrack_0 (Timeline|Timeline Play)
    (:Update
      (Transformation|SetActorTransform (Math|Transform|Lerp(Transform) (Variables|Default|GetTransformA) (Math|Transform|MakeTransform (+ (.location _transformb) (.location _transforma)) (Math|Rotator|MakeRotator (+ _roll _roll_2) (+ _pitch _pitch_2) (+ _yaw _yaw_2)) (.scale _transformb)) _newtrack_0)))))

(event EventBeginPlay
  (Variables|Default|SetTransformA (Transformation|GetActorTransform)))

(fn ConstructionScript
  (|CallParentFunction))