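; BP_HandObject is an interactable hand-equipment object in the equipment system, with its mesh defined by data.
; The construction script looks up the HandData row in its data table and applies that row's static mesh.
; The focus interface event toggles custom depth rendering on the mesh, and a getter exposes its Widget.
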(event EventInterfaceToggleFocus
  (params (Focus :type Boolean))
  (Rendering|SetRenderCustomDepth (Variables|Default|GetStaticMesh) Focus))

(fn ConstructionScript
  (bind _handdata (Variables|Default|GethandData))
  (bind _returnvalue (Utilities|GetDataTableRow (.datatable _handdata) (.rowname _handdata))
    (:then
      (Utilities|FlowControl|Sequence
        (:then_0
          (Components|StaticMesh|SetStaticMesh (Variables|Default|GetStaticMesh) (.StaticMesh (Utilities|Struct|BreakS_Hands _returnvalue))))))))

(fn GetWidget
  (return (Variables|Default|GetWidget)))