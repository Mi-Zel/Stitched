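; An interactable lever that checks the solution to a lever puzzle and opens a gate.
; On primary interaction it compares the current and correct states of every BP_Child_HandLeverLight tagged PuzzleLever, stopping at the first mismatch.
; If all match, it triggers the first BP_Gate2 tagged lastHopeGate through BI_InteractedTarget.
; Otherwise it shows a timed incorrect-sequence warning on the HUD.
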(event EventBeginPlay)

(event Collision|EventActorBeginOverlap
  (params (OtherActor :type Actor%20Object%20Reference)))

(event EventTick
  (params (DeltaSeconds :type Float%20%28single-precision%29)))

(event EventPrimaryInteract
  (bind _outactors (Actor|GetAllActorsOfClasswithTag "/Game/Interaction/InteractionArea/BP_Child_HandLeverLight.BP_Child_HandLeverLight_C" "PuzzleLever"))
  (bind _array_element (Utilities|Array|ForEachLoopwithBreak _outactors :!label _label)
    (:LoopBody
      (bind _asbp_child_hand_lever_light (Utilities|Casting|CastToBP_Child_HandLeverLight _array_element))
      (bind _output_get (Variables|Default|SetResult (== (Variables|/Game/Interaction/InteractionArea/BP_Child_HandLeverLight.BP_Child_HandLeverLight_C|GetCorrect _asbp_child_hand_lever_light) (Variables|/Game/Interaction/InteractionArea/BP_Child_HandLeverLight.BP_Child_HandLeverLight_C|GetcurrentState _asbp_child_hand_lever_light))))
      (if (not _output_get)
        (goto _label Break)))
    (:Completed
      (if (Variables|Default|GetResult)
        (bind _outactors_2 (Actor|GetAllActorsOfClasswithTag "/Game/Interaction/BP_Gate2.BP_Gate2_C" "lastHopeGate"))
        (bind _asbi_interacted_target (Utilities|Casting|CastToBI_InteractedTarget (Utilities|Array|Get(acopy) _outactors_2)))
        (Default|PrimaryInteract _asbi_interacted_target)
        (else
          (bind _returnvalue (Actor|GetActorOfClass (Variables|/Script/Engine.GameModeBase|GetHUDClass (Game|GetGameMode))))
          (bind _asbp_hud_core (Utilities|Casting|CastToBP_HUD_Core _returnvalue))
          (Default|HUDWarningMessage (Variables|/Game/Core/BP_HUD_Core.BP_HUD_Core_C|GetWB_HUD _asbp_hud_core) "Incorrect Sequence" 5.0))))))

(fn ConstructionScript
  (|CallParentFunction))

(fn GetWidget
  (return (Variables|Default|GetWidget)))