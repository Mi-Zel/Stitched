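; BP_InteractionArea is an interaction area actor that relays focus changes to its parent actor.
; ToggleFocus stores the focus state, forwards it to the parent through InterfaceToggleFocusMessage, and shows or hides the parent's message widget to match.
; On BeginPlay it copies InteractionTarget from the parent into TargetInteraction, which works only when the parent is a BP_TestInteractionActor.
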(event Custom|Toggle%20Focus
  (params (Focused :type Boolean))
  (bind _returnvalue (Actor|GetParentActor))
  (bind _output_get (Variables|Default|SetFocused Focused))
  (Utilities|FlowControl|Sequence
    (:then_0
      (Class|BIInteraction|InterfaceToggleFocus(Message) _returnvalue _output_get))
    (:then_1
      (bind _ref (Class|BIInteraction|GetWidget(Message) _returnvalue))
      (Development|SetHiddeninGame _ref (not _output_get) false))))

(event EventBeginPlay
  (bind _asbp_test_interaction_actor (Utilities|Casting|CastToBP_TestInteractionActor (Actor|GetParentActor)))
  (Variables|Default|Settarget%20interaction (Variables|/Game/Interaction/BP_TestInteractionActor.BP_TestInteractionActor_C|Getinteraction%20target _asbp_test_interaction_actor)))

(fn ConstructionScript)